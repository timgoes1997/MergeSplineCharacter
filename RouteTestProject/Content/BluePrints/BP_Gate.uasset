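; BP_Gate is a gate actor that stores a forced scale, a thermal value and a gate number.
; Simple setter functions write each of these values.
; On BeginPlay it applies the forced world scale to GateMesh, then prints the thermal value, number, forced scale and resulting mesh scale as debug text.
; The construction script is empty, so the scale takes effect only when play begins.
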(event EventBeginPlay
  (Transformation|SetWorldScale3D (Variables|Default|GetGateMesh) (Variables|Default|GetForcedScale))
  (Development|PrintText (Utilities|Text|ToText(Float) (Variables|Default|GetGateThermal) "HalfToEven") true true "(R=0.000000,G=0.660000,B=1.000000,A=1.000000)" 2e+01)
  (Development|PrintText (Utilities|Text|ToText(Integer) (Variables|Default|GetGateNumber)) true true "(R=0.000000,G=0.660000,B=1.000000,A=1.000000)" 2e+01)
  (Development|PrintText (Utilities|Text|ToText(String) (Variables|Default|GetForcedScale)) true true "(R=0.000000,G=0.660000,B=1.000000,A=1.000000)" 2e+01)
  (Development|PrintText (Utilities|Text|ToText(String) (Transformation|GetWorldScale (Variables|Default|GetGateMesh))) true true "(R=0.000000,G=0.660000,B=1.000000,A=1.000000)" 2e+01))

(event Collision|EventActorBeginOverlap
  (params (OtherActor :type Actor%20Object%20Reference)))

(event EventTick
  (params (DeltaSeconds :type Float%20%28single-precision%29)))

(fn ConstructionScript)

(fn SetForceScale
  (params (Scale :type Vector))
  (Variables|Default|SetForcedScale Scale))

(fn SetThermal
  (params (Thermal :type Float%20%28single-precision%29))
  (Variables|Default|SetGateThermal Thermal))

(fn SetGateNumber
  (params (GateNumber :type Integer))
  (Variables|Default|SetGateNumber GateNumber))