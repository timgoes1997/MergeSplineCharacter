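; Spline-based route generator that builds a track mesh and optional numbered gates in its construction script.
; It resizes a per-point route data array to match the spline point count, then adds a collision-toggleable spline mesh per segment, blending each point's width and thickness and optionally closing the loop.
; Points flagged for gates get BP_Gate child actors oriented against the spline tangent, receiving scale, thermal setting and gate number.
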(event EventBeginPlay)

(event Collision|EventActorBeginOverlap
  (params (OtherActor :type Actor%20Object%20Reference)))

(event EventTick
  (params (DeltaSeconds :type Float%20%28single-precision%29)))

(fn ConstructionScript
  (Utilities|FlowControl|Sequence
    (:then_0
      (|Getthenumberofsplinepoints))
    (:then_1
      (|BuildRouteDataArray))
    (:then_2
      (bind _index (|SplineLoop)
        (:LoopBody
          (CallFunction|BuildRouteElement _index (Variables|RouteMeshes|GetRouteMesh)))))
    (:then_3
      (|SpawnGates))))

(fn BuildRouteElement
  (params (Loop%20index :type Integer) (RouteElementMesh :type Static%20Mesh%20Object%20Reference))
  (LocalVariables|SetLocalCurrentLoopIndex Loop%20index)
  (LocalVariables|SetLocalNextLoopIndex (Math|Integer|%(Integer) (+ Loop%20index 1) (Variables|Spline|GetNumberOfSplinePoints)))
  (LocalVariables|SetLocalRouteElementMesh RouteElementMesh)
  (Utilities|FlowControl|Sequence
    (:then_0
      (LocalVariables|SetLocalStartLocation (.Location (Spline|GetLocationandTangentatSplinePoint (Variables|Default|GetSpline) (LocalVariables|GetLocalCurrentLoopIndex) "Local")))
      (LocalVariables|SetLocalStartTangent (.Tangent (Spline|GetLocationandTangentatSplinePoint (Variables|Default|GetSpline) (LocalVariables|GetLocalCurrentLoopIndex) "Local")))
      (LocalVariables|SetLocalEndLocation (.Location (Spline|GetLocationandTangentatSplinePoint (Variables|Default|GetSpline) (LocalVariables|GetLocalNextLoopIndex) "Local")))
      (LocalVariables|SetLocalEndTangent (.Tangent (Spline|GetLocationandTangentatSplinePoint (Variables|Default|GetSpline) (LocalVariables|GetLocalNextLoopIndex) "Local")))
      (LocalVariables|SetLocalStartScale (Math|Vector2D|MakeVector2D (.routewidth (Utilities|Array|Get(acopy) (Variables|RouteSetup|GetRouteDataArray) (LocalVariables|GetLocalCurrentLoopIndex))) (.routethickness (Utilities|Array|Get(acopy) (Variables|RouteSetup|GetRouteDataArray) (LocalVariables|GetLocalCurrentLoopIndex)))))
      (LocalVariables|SetLocalEndScale (Math|Vector2D|MakeVector2D (.routewidth (Utilities|Array|Get(acopy) (Variables|RouteSetup|GetRouteDataArray) (LocalVariables|GetLocalNextLoopIndex))) (.routethickness (Utilities|Array|Get(acopy) (Variables|RouteSetup|GetRouteDataArray) (LocalVariables|GetLocalNextLoopIndex))))))
    (:then_1
      (bind _returnvalue (AddComponent|AddSplineMeshComponent false))
      (LocalVariables|SetLocalCurrentSplineMesh _returnvalue)
      (Components|StaticMesh|SetStaticMesh (LocalVariables|GetLocalCurrentSplineMesh) (LocalVariables|GetLocalRouteElementMesh))
      (SplineMesh|SetStartandEnd (LocalVariables|GetLocalCurrentSplineMesh) (LocalVariables|GetLocalStartLocation) (LocalVariables|GetLocalStartTangent) (LocalVariables|GetLocalEndLocation) (LocalVariables|GetLocalEndTangent) true :!class /Script/Engine.SplineMeshComponent)
      (SplineMesh|SetStartScale (LocalVariables|GetLocalCurrentSplineMesh) (LocalVariables|GetLocalStartScale) true :!class /Script/Engine.SplineMeshComponent)
      (SplineMesh|SetEndScale (LocalVariables|GetLocalCurrentSplineMesh) (LocalVariables|GetLocalEndScale) true :!class /Script/Engine.SplineMeshComponent)
      (Collision|SetCollisionEnabled (LocalVariables|GetLocalCurrentSplineMesh) (select (Variables|Collision|GetCollisions) "QueryAndPhysics" "NoCollision")))))